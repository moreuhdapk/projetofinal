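; BP_FPSplayer is the first-person player pawn for the retro FPS, handling HUD creation, movement and mouse look.
; On BeginPlay it creates the BP_hud widget and adds it to the viewport.
; Movement axes feed AddMovementInput using right and forward vectors built only from control yaw, so pitch does not affect direction.
; Mouse-look axes feed controller yaw and pitch directly.
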(event EventBeginPlay
  (bind _returnvalue (UserInterface|CreateWidget "/Game/retroFps/blueprints/BP_hud.BP_hud_C"))
  (UserInterface|Viewport|AddtoViewport _returnvalue 0))

(event Input|AxisEvents|InputAxisverticalmovement
  (params (AxisValue :type Float%20%28single-precision%29))
  (Pawn|Input|AddMovementInput (Math|Vector|GetForwardVector (Math|Rotator|MakeRotator 0.0 0.0 (.yaw (Pawn|GetControlRotation :!class /Script/Engine.Pawn)))) AxisValue false))

(event Input|AxisEvents|InputAxishorizontalmovement
  (params (AxisValue :type Float%20%28single-precision%29))
  (Pawn|Input|AddMovementInput (Math|Vector|GetRightVector (Math|Rotator|MakeRotator 0.0 0.0 (.yaw (Pawn|GetControlRotation :!class /Script/Engine.Pawn)))) AxisValue false))

(event Input|AxisEvents|InputAxismouselookHorizontal
  (params (AxisValue :type Float%20%28single-precision%29))
  (Pawn|Input|AddControllerYawInput AxisValue))

(event Input|AxisEvents|InputAxismouuselookvertical
  (params (AxisValue :type Float%20%28single-precision%29))
  (Pawn|Input|AddControllerPitchInput AxisValue))

(fn ConstructionScript)